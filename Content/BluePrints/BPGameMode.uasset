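; Game mode that procedurally generates and spawns a tile-based maze at BeginPlay.
; InitWorld fills a flat, XY-indexed array with ground on even-even cells and walls elsewhere.
; RandomizeWorld carves binary-tree style, opening a random +X or +Y wall beside each ground cell, with fallbacks when neither is a wall.
; SpawnWorld then places ground or wall actors on a 200-unit grid, with debug prints along the way.
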(event EventBeginPlay
  (CallFunction|InitWorld)
  (CallFunction|RandomizeWorld)
  (CallFunction|SpawnWorld))

(event EventTick
  (params (DeltaSeconds :type Float%20%28single-precision%29)))

(fn ConstructionScript)

(fn IsTileEmpty
  (params (X :type Integer) (Y :type Integer))
  (bind _valid (CallFunction|CheckTileLocation X Y))
  (if _valid
    (bind _index (CallFunction|XY2Index X Y))
    (return (Utilities|Enum|Equal(Enum) (Utilities|Array|Get(acopy) (Variables|Default|GetTilesLevel) _index) "NewEnumerator0"))
    (else
      (return false))))

(fn SetTileStatus
  (params (X :type Integer) (Y :type Integer) (empty :type ENUMTileState%20Enum))
  (bind _valid (CallFunction|CheckTileLocation X Y))
  (if _valid
    (bind _index (CallFunction|XY2Index X Y))
    (Utilities|Array|SetArrayElem (Variables|Default|GetTilesLevel) _index empty)
    (return)
    (else
      (return))))

(fn CheckTileLocation
  (params (x :type Integer) (y :type Integer))
  (return (Math|Boolean|ANDBoolean (>= x (Variables|Default|GetMinX)) (< x (Variables|Default|GetMaxX)) (>= y (Variables|Default|GetMinY)) (< y (Variables|Default|GetMaxY)))))

(fn GetTileStatus
  (params (X :type Integer) (Y :type Integer))
  (bind _valid (CallFunction|CheckTileLocation X Y))
  (if _valid
    (bind _index (CallFunction|XY2Index X Y))
    (return (Utilities|Array|Get(acopy) (Variables|Default|GetTilesLevel) _index))
    (else
      (return "NewEnumerator6"))))

(fn Index2Transform
  (params (index :type Integer))
  (bind _location (CallFunction|Index2Vector index))
  (return (Math|Transform|MakeTransform _location "0, 0, 0" "1.000000,1.000000,1.000000")))

(fn InitWorld
  (bind _tileslevel (Variables|Default|GetTilesLevel))
  ;[1 1 1] Compute world size
  (bind _output_get (Variables|Default|SetDeltaX (Math|Float|Truncate (|(abs((Max-Min))) (Math|Conversions|ToFloat(Integer) (Variables|Default|GetMaxX)) (Math|Conversions|ToFloat(Integer) (Variables|Default|GetMinX))))))
  (bind _output_get_2 (Variables|Default|SetDeltaY (Math|Float|Truncate (|(abs((Max-Min))) (Math|Conversions|ToFloat(Integer) (Variables|Default|GetMaxY)) (Math|Conversions|ToFloat(Integer) (Variables|Default|GetMinY))))))
  (bind _output_get_3 (Variables|Default|SetLinearSize (* _output_get _output_get_2)))
  ;[1 1 1] Initialize IsEmpty
  (Utilities|Array|Resize _tileslevel _output_get_3)
  (for (_ _array_index) _tileslevel
    (bind (_x _y) (CallFunction|Index2XY _array_index))
    (if (and (== (Math|Integer|%(Integer) _x 2) 0) (== (Math|Integer|%(Integer) _y 2) 0))
      (Utilities|Array|SetArrayElem _tileslevel _array_index "NewEnumerator0")
      (else
        (Utilities|Array|SetArrayElem _tileslevel _array_index "NewEnumerator1"))))
  ;[1 1 1] Debug Output
  (Development|PrintText (Utilities|Text|FormatText "({dx}, {dy}) size {total}" (Utilities|Text|ToText(Integer) (Variables|Default|GetDeltaX)) (Utilities|Text|ToText(Integer) (Variables|Default|GetDeltaY)) (Utilities|Text|ToText(Integer) (Variables|Default|GetLinearSize))) true true "(R=0.000000,G=0.660000,B=1.000000,A=1.000000)" 1.2e+02))

(fn SpawnWorld
  (for (_array_element _array_index) (Variables|Default|GetTilesLevel)
    (bind _transform (CallFunction|Index2Transform _array_index))
    (switch Utilities|FlowControl|Switch|SwitchonENUMTileState _array_element
      (:NewEnumerator0
        (Game|SpawnActorfromClass "/Game/BluePrints/BPEmtpyTile.BPEmtpyTile_C" _transform "AlwaysSpawn" 0 0)
        (Development|PrintText "Ground"))
      (:NewEnumerator1
        (Game|SpawnActorfromClass "/Game/BluePrints/BPWallTile.BPWallTile_C" _transform "AlwaysSpawn" 0 0)
        (Development|PrintText "Wall")))))

(fn Index2XY
  (params (Index :type Integer))
  (bind _maxx (Variables|Default|GetMaxX))
  (bind _maxx_2 (Variables|Default|GetMaxX))
  (bind _returnvalue (/ Index _maxx))
  (bind _returnvalue_2 (Math|Integer|%(Integer) Index _maxx_2))
  (if (> Index (Variables|Default|GetLinearSize))
    (Development|PrintText "Error Index out of bounds" true true "(R=1.000000,G=0.000000,B=0.036710,A=1.000000)")
    (else
      (Development|PrintText (Utilities|Text|FormatText "{X}, {Y}" (Utilities|Text|ToText(Integer) _returnvalue_2) (Utilities|Text|ToText(Integer) _returnvalue)))))
  (return _returnvalue_2 _returnvalue))

(fn Index2Vector
  (params (Index :type Integer))
  (bind (_x _y) (CallFunction|Index2XY Index))
  (return (Math|Vector|MakeVector (* _x 2e+02) (* _y 2e+02) 0.0)))

(fn RandomizeWorld
  (for (_ _array_index) (Variables|Default|GetTilesLevel)
    (bind (_x _y) (CallFunction|Index2XY _array_index))
    (bind _output_get (LocalVariables|SetlocalX _x))
    (bind _output_get_2 (LocalVariables|SetlocalY _y))
    (if (and (== (Math|Integer|%(Integer) _output_get 2) 0) (== (Math|Integer|%(Integer) _output_get_2 2) 0))
      (bind (_aroundstatus _aroundx _aroundy) (CallFunction|GetTileAroundStatus (LocalVariables|GetlocalX) (LocalVariables|GetlocalY)))
      (bind _output_get_3 (LocalVariables|SetrandomIndex (Math|Random|RandomInteger 2)))
      (if (Utilities|Enum|Equal(Enum) (Utilities|Array|Get(acopy) _aroundstatus _output_get_3) "NewEnumerator1")
        _
        (else
          (bind _output_get_4 (LocalVariables|SetrandomIndex (Math|Integer|%(Integer) (+ (LocalVariables|GetrandomIndex) 1) 2)))
          (if (Utilities|Enum|Equal(Enum) (Utilities|Array|Get(acopy) _aroundstatus _output_get_4) "NewEnumerator1")
            _
            (else
              (bind _output_get_5 (LocalVariables|SetrandomIndex (+ (LocalVariables|GetrandomIndex) 2)))
              (if (Utilities|Enum|Equal(Enum) (Utilities|Array|Get(acopy) _aroundstatus _output_get_5) "NewEnumerator1")
                _
                (elif true
                  (LocalVariables|SetrandomIndex 2)
                  (else
                    (LocalVariables|SetrandomIndex 3))))))))
      (CallFunction|SetTileStatus (Utilities|Array|Get(acopy) _aroundx (LocalVariables|GetrandomIndex)) (Utilities|Array|Get(acopy) _aroundy (LocalVariables|GetrandomIndex)) "NewEnumerator0"))))

(fn XY2Index
  (params (X :type Integer) (Y :type Integer))
  (return (+ X (* Y (Variables|Default|GetMaxX)))))

(fn GetTileAroundStatus
  (params (X :type Integer) (Y :type Integer))
  (bind _returnvalue (+ X 1))
  (bind _returnvalue_2 (+ Y -1))
  (bind _returnvalue_3 (+ Y 1))
  (bind _returnvalue_4 (+ X -1))
  (Utilities|Array|Resize (LocalVariables|GetoutStatus) 4)
  (Utilities|Array|Resize (LocalVariables|GetoutX) 4)
  (Utilities|Array|Resize (LocalVariables|GetoutY) 4)
  (bind _newparam (CallFunction|GetTileStatus _returnvalue Y))
  (Utilities|Array|SetArrayElem (LocalVariables|GetoutStatus) 0 _newparam)
  (Utilities|Array|SetArrayElem (LocalVariables|GetoutX) 0 _returnvalue)
  (Utilities|Array|SetArrayElem (LocalVariables|GetoutY) 0 Y)
  (bind _newparam_2 (CallFunction|GetTileStatus X _returnvalue_3))
  (Utilities|Array|SetArrayElem (LocalVariables|GetoutStatus) 1 _newparam_2)
  (Utilities|Array|SetArrayElem (LocalVariables|GetoutX) 1 X)
  (Utilities|Array|SetArrayElem (LocalVariables|GetoutY) 1 _returnvalue_3)
  (bind _newparam_3 (CallFunction|GetTileStatus _returnvalue_4 Y))
  (Utilities|Array|SetArrayElem (LocalVariables|GetoutStatus) 2 _newparam_3)
  (Utilities|Array|SetArrayElem (LocalVariables|GetoutX) 2 _returnvalue_4)
  (Utilities|Array|SetArrayElem (LocalVariables|GetoutY) 2 Y)
  (bind _newparam_4 (CallFunction|GetTileStatus X _returnvalue_2))
  (Utilities|Array|SetArrayElem (LocalVariables|GetoutStatus) 3 _newparam_4)
  (Utilities|Array|SetArrayElem (LocalVariables|GetoutX) 3 X)
  (Utilities|Array|SetArrayElem (LocalVariables|GetoutY) 3 _returnvalue_2)
  (return (LocalVariables|GetoutStatus) (LocalVariables|GetoutX) (LocalVariables|GetoutY)))