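; Player controller for grid-based, step-by-step movement of BPPlayerPawn with 90-degree turns.
; Forward and backward inputs compute a target one tile away along the facing direction and ask BPGameMode whether it is empty.
; Free tiles trigger a timeline transform lerp, while blocked ones print a hit message.
; Turn inputs lerp yaw on a second timeline, and a Moving flag ignores input until each action ends.
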(event `self.ReceiveBeginPlay`)

(event `self.ReceiveTick`
  (params (DeltaSeconds :type "Float (single-precision)")))

(event `InputAction|MoveForward`
  (params (Key :type "Key Structure" :default "AnyKey"))
  (bind _returnvalue (`KismetMathLibrary.FTrunc` (/ (.x (.location (`self.TransformTo`))) 199.0)))
  (bind _returnvalue_2 (`KismetMathLibrary.FTrunc` (/ (.y (.location (`self.TransformTo`))) 199.0)))
  (:`Pressed`
    (if (not (`self.moving`))
      (set `self.moving` true)
      ;[1 1 1] Forward
      (bind _asbpplayer_pawn (cast `/Game/Blueprints/BPPlayerPawn` (`GameplayStatics.GetPlayerPawn` 0)))
      (`self.UpdateVariables`)
      (bind _output_get (set `self.TransformFrom` (`self.GetTransform` _asbpplayer_pawn)))
      (set `self.TransformTo` (`KismetMathLibrary.MakeTransform` (+ (.location _output_get) (* (`self.ForwardDirection`) 200)) (.rotation _output_get) (.scale _output_get)))
      ;[1 1 1] Check Collision
      (bind _asbpgame_mode (cast `/Game/Blueprints/BPGameMode` (`GameplayStatics.GetGameMode`) :!label _label))
      (bind _out (`/Game/Blueprints/BPGameMode.IsTileEmpty` _asbpgame_mode _returnvalue _returnvalue_2))
      (`KismetSystemLibrary.PrintText` (`|FormatText` "player ({px}, {py}) dest ({dx}, {dy})" (`KismetTextLibrary.Conv_IntToText` (`self.playerX`)) (`KismetTextLibrary.Conv_IntToText` (`self.playerY`)) (`KismetTextLibrary.Conv_IntToText` _returnvalue) (`KismetTextLibrary.Conv_IntToText` _returnvalue_2)))
      (if _out
        ;[1 1 1] Move
        (bind (_direction _newtrack_0) (`Timeline|TimeLineMove` :!via `PlayFromStart`)
          (:`Update`
            (bind _asbpplayer_pawn_2 (cast `/Game/Blueprints/BPPlayerPawn` (`GameplayStatics.GetPlayerPawn` 0)))
            (`self.K2_SetActorTransform` _asbpplayer_pawn_2 (`KismetMathLibrary.TLerp` (`self.TransformFrom`) (`self.TransformTo`) _newtrack_0) true false))
          (:`Finished`
            (set `self.moving` false)))
        (else
          (set `self.moving` false)
          (`KismetSystemLibrary.PrintText` "Hit" true true (struct :`R` 1.0 :`A` 1.0)))))))

(event `InputAction|MoveBackward`
  (params (Key :type "Key Structure" :default "AnyKey"))
  (:`Pressed`
    (if (not (`self.moving`))
      (set `self.moving` true)
      ;[1 1 1] Backward
      (bind _asbpplayer_pawn (cast `/Game/Blueprints/BPPlayerPawn` (`GameplayStatics.GetPlayerPawn` 0)))
      (`self.UpdateVariables`)
      (bind _output_get (set `self.TransformFrom` (`self.GetTransform` _asbpplayer_pawn)))
      (set `self.TransformTo` (`KismetMathLibrary.MakeTransform` (- (.location _output_get) (* (`self.ForwardDirection`) 200)) (.rotation _output_get) (.scale _output_get)))
      (goto _label))))

(event `InputAction|TurnRight`
  (params (Key :type "Key Structure" :default "AnyKey"))
  (:`Pressed`
    (if (not (`self.moving`))
      (set `self.moving` true)
      ;[1 1 1] Right
      (bind _asbpplayer_pawn (cast `/Game/Blueprints/BPPlayerPawn` (`GameplayStatics.GetPlayerPawn` 0)))
      (bind _returnvalue (`self.K2_GetActorRotation` _asbpplayer_pawn))
      (set `self.RotateFrom` _returnvalue)
      (set `self.RotateTo` (`KismetMathLibrary.MakeRotator` 0.0 0.0 (+ (.yaw _returnvalue) 90.0)))
      ;[1 1 1] Rotate
      (bind (_direction _newtrack_0) (`Timeline|TimelineTurn` :!via `PlayFromStart` :!label _label_2)
        (:`Update`
          (bind _asbpplayer_pawn_2 (cast `/Game/Blueprints/BPPlayerPawn` (`GameplayStatics.GetPlayerPawn` 0)))
          (`self.SetActorRotation` _asbpplayer_pawn_2 (`KismetMathLibrary.RLerp` (`self.RotateFrom`) (`self.RotateTo`) _newtrack_0)))
        (:`Finished`
          (set `self.moving` false))))))

(event `InputAction|TurnLeft`
  (params (Key :type "Key Structure" :default "AnyKey"))
  (:`Pressed`
    (if (not (`self.moving`))
      (set `self.moving` true)
      ;[1 1 1] Left
      (bind _asbpplayer_pawn (cast `/Game/Blueprints/BPPlayerPawn` (`GameplayStatics.GetPlayerPawn` 0)))
      (bind _returnvalue (`self.K2_GetActorRotation` _asbpplayer_pawn))
      (set `self.RotateFrom` _returnvalue)
      (set `self.RotateTo` (`KismetMathLibrary.MakeRotator` 0.0 0.0 (+ (.yaw _returnvalue) -90.0)))
      (goto _label_2 :!via `PlayFromStart`))))

(fn `UpdateVariables`
  (bind _returnvalue (`GameplayStatics.GetPlayerPawn` 0))
  (set `self.playerX` (`KismetMathLibrary.FTrunc` (/ (.x (`self.K2_GetActorLocation` _returnvalue)) 200.0)))
  (set `self.playerY` (`KismetMathLibrary.FTrunc` (/ (.y (`self.K2_GetActorLocation` _returnvalue)) 200.0)))
  (set `self.ForwardDirection` (`KismetMathLibrary.Normal` (`self.GetActorForwardVector` _returnvalue)))
  (set `self.PlayerPawnLocation` (`self.K2_GetActorLocation` _returnvalue)))

(fn `UserConstructionScript`)